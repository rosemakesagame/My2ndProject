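; BP_BigTree is an interactable tree that the player decorates with mushrooms from the inventory.
; Its trigger sphere registers the tree as the character's CurrentBigTree and, when the GI_MyGame inventory has items, shows a decor prompt and notification, undone on exit except the notification.
; PreviewTree displays the selected Forest item's mesh on MushroomDecor.
; ConfirmDecorate, once previewed, clears the entire inventory and refreshes the hotbar, leaving the mesh in place.
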(event `self.ReceiveBeginPlay`
  ; HUD
  (bind _aswbp_interaction_prompt (cast `/Game/BP/WBP_InteractionPrompt` (`WidgetComponent.GetUserWidgetObject` (`self.PromptWidget`))))
  (`/Game/BP/WBP_InteractionPrompt.SetPromptText` _aswbp_interaction_prompt "[1,2,3] Select | [F] Preview | [E] Confirm"))

(event `self.TriggerSphere.OnComponentBeginOverlap`
  (params (OverlappedComponent :type "PrimitiveComponent Object Reference") (OtherActor :type "Actor Object Reference") (OtherComp :type "PrimitiveComponent Object Reference") (OtherBodyIndex :type Integer) (bFromSweep :type Boolean) (SweepResult :type "HitResult Structure (by ref)"))
  (bind _asbp_first_person_character (cast `/Game/FirstPerson/Blueprints/BP_FirstPersonCharacter` OtherActor))
  (set `/Game/FirstPerson/Blueprints/BP_FirstPersonCharacter.CurrentBigTree` self _asbp_first_person_character)
  (bind _asgi_my_game (cast `/Game/BP/GI_MyGame` (`GameplayStatics.GetGameInstance`)))
  (if (> (`KismetArrayLibrary.Array_Length` (`/Game/BP/GI_MyGame.Inventory` _asgi_my_game)) 0)
    (bind _returnvalue (`|CreateWidget` "/Game/BP/WBP_TreeDecorPrompt.WBP_TreeDecorPrompt_C"))
    (bind _output_get (set `self.ActiveDecorWidget` _returnvalue))
    (`UserWidget.AddToViewport` _output_get 0)
    (`/Game/BP/WBP_NotificationToast.ShowNotification` (`/Game/FirstPerson/Blueprints/BP_FirstPersonCharacter.NotificationWidget` _asbp_first_person_character) "It's time to decorate the tree! \nSelect a mushroom and decorate the tree!")))

(event `self.TriggerSphere.OnComponentEndOverlap`
  (params (OverlappedComponent :type "PrimitiveComponent Object Reference") (OtherActor :type "Actor Object Reference") (OtherComp :type "PrimitiveComponent Object Reference") (OtherBodyIndex :type Integer))
  (bind _activedecorwidget (`self.ActiveDecorWidget`))
  (bind _asbp_first_person_character (cast `/Game/FirstPerson/Blueprints/BP_FirstPersonCharacter` OtherActor))
  (set `/Game/FirstPerson/Blueprints/BP_FirstPersonCharacter.CurrentBigTree` null _asbp_first_person_character)
  (`/Engine/EditorBlueprintResources/StandardMacros.IsValid` _activedecorwidget
    (:`Is Valid`
      (`Widget.RemoveFromParent` _activedecorwidget)
      (set `self.ActiveDecorWidget` null))))

(event `PreviewTree`
  ; PreviewTree
  (bind _asgi_my_game (cast `/Game/BP/GI_MyGame` (`GameplayStatics.GetGameInstance`)))
  (bind _inventory (`/Game/BP/GI_MyGame.Inventory` _asgi_my_game))
  (if (> (`KismetArrayLibrary.Array_Length` _inventory) 0)
    (bind (_output_itemname _output_itemicon _output_itemtype _output_itemmesh) (break `/Game/BP/F_ItemData` (`|GetArrayItem` _inventory (`/Game/BP/GI_MyGame.SelectedIndex` _asgi_my_game))))
    (switch `/Game/BP/E_ItemType` _output_itemtype
      (:`NewEnumerator0`
        (`StaticMeshComponent.SetStaticMesh` (`self.MushroomDecor`) _output_itemmesh)
        (`SceneComponent.SetVisibility` (`self.MushroomDecor`) true false)
        (set `self.IsPreviewed` true)))))

(event `ConfirmDecorate`
  ; ConfirmDecorate
  (bind _asgi_my_game (cast `/Game/BP/GI_MyGame` (`GameplayStatics.GetGameInstance`)))
  (if (`self.IsPreviewed`)
    (`KismetArrayLibrary.Array_Clear` (`/Game/BP/GI_MyGame.Inventory` _asgi_my_game))
    (bind _asbp_first_person_character (cast `/Game/FirstPerson/Blueprints/BP_FirstPersonCharacter` (`GameplayStatics.GetPlayerCharacter` 0)))
    (`/Game/BP/WBP_Hotbar.RefreshHotbar` (`/Game/FirstPerson/Blueprints/BP_FirstPersonCharacter.HotbarWidget` _asbp_first_person_character))
    (set `self.IsPreviewed` false)))

(fn `UserConstructionScript`)